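; GameStateDealer tracks the in-game clock and the player's suspicion level for a dealing game.
; Each Tick advances Time, stored in minutes, by a debug time scale, and raises Suspicion during a deal or lowers it otherwise, without clamping.
; Helpers convert between minutes, hours and days, build the displayed clock text using day names from GameModeDealer, and skip to 9:00 the next day.
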(event `self.ReceiveBeginPlay`
  (bind _asfirst_person_character (cast `/Game/Assets/Blueprints/FirstPersonCharacter` (`GameplayStatics.GetPlayerPawn` 0)))
  (set `self.Player` _asfirst_person_character))

(event `self.ReceiveTick`
  (params (DeltaSeconds :type "Float (single-precision)"))
  (set `self.DeltaTime` DeltaSeconds)
  (`self.UpdateTime`)
  (`self.UpdateSuspision`)
  (bind _output (`self.TimeToText` (`self.Time`)))
  (set `self.TextTime` _output))

(fn `DaysToMinutes`
  (params (Days :type Integer))
  (returns (Minutes :type "Float (double-precision)"))
  (return (`KismetMathLibrary.Conv_IntToDouble` (* Days (* 60 24)))))

(fn `ExtractHours`
  (params (Time :type "Float (double-precision)"))
  (returns (Hours :type Integer))
  (bind _days (`self.MinutesToDays` Time true))
  (bind _minutes (`self.DaysToMinutes` (`KismetMathLibrary.FTrunc` _days)))
  (bind _hours (`self.MinutesToHours` (- Time _minutes) true))
  (return (`KismetMathLibrary.FTrunc` _hours)))

(fn `ExtractMinutes`
  (params (Time :type "Float (double-precision)"))
  (returns (Minutes :type Integer))
  (bind _days (`self.MinutesToDays` Time true))
  (bind _minutes (`self.DaysToMinutes` (`KismetMathLibrary.FTrunc` _days)))
  (bind _returnvalue (- Time _minutes))
  (bind _hours (`self.ExtractHours` _returnvalue))
  (bind _minutes_2 (`self.HoursToMinutes` _hours))
  (return (`KismetMathLibrary.FTrunc` (- _returnvalue _minutes_2))))

(fn `GoToNextDay`
  (bind _days (`self.MinutesToDays` (`self.Time`) true))
  (bind _result (`/Engine/EditorBlueprintResources/StandardMacros.IncrementInt` (`KismetMathLibrary.FTrunc` _days))
    (:`  `
      (bind _minutes (`self.DaysToMinutes` _result))
      (bind _minutes_2 (`self.HoursToMinutes` 9))
      (set `self.Time` (+ _minutes _minutes_2)))))

(fn `HoursToMinutes`
  (params (Hours :type Integer))
  (returns (Minutes :type "Float (double-precision)"))
  (return (* Hours 60.0)))

(fn `InitState`
  (set `self.Suspicion` 0.0)
  (set `self.Time` (* 60.0 9.0)))

(fn `MinutesToDays`
  (params (Minutes :type "Float (double-precision)") (Round :type Boolean))
  (returns (Days :type "Float (double-precision)"))
  (bind _returnvalue (/ Minutes (* 60.0 24.0)))
  (if Round
    (return (`KismetMathLibrary.Conv_IntToDouble` (`KismetMathLibrary.FTrunc` _returnvalue)))
    (else
      (return _returnvalue))))

(fn `MinutesToHours`
  (params (Minutes :type "Float (double-precision)") (Round :type Boolean))
  (returns (Hours :type "Float (double-precision)"))
  (bind _returnvalue (/ Minutes 60.0))
  (if Round
    (return (`KismetMathLibrary.Conv_IntToDouble` (`KismetMathLibrary.FTrunc` _returnvalue)))
    (else
      (return _returnvalue))))

(fn `TimeToText`
  (params (Time :type "Float (double-precision)"))
  (returns (Output :type String))
  (bind _days (`self.MinutesToDays` Time true))
  (bind _minutes (`self.DaysToMinutes` (`KismetMathLibrary.FTrunc` _days)))
  (bind _returnvalue (- Time _minutes))
  (bind _hours (`self.MinutesToHours` _returnvalue true))
  (bind _minutes_2 (`self.HoursToMinutes` (`KismetMathLibrary.FTrunc` _hours)))
  (bind _asgame_mode_dealer (cast `/Game/Assets/Blueprints/GameModeDealer` (`GameplayStatics.GetGameMode`)))
  (bind _name (`/Game/Assets/Blueprints/GameModeDealer.GetDayName` _asgame_mode_dealer (`KismetMathLibrary.Conv_IntToDouble` (`KismetMathLibrary.FTrunc` _days))))
  (return (`KismetStringLibrary.Concat_StrStr` _name " - " (`KismetStringLibrary.Conv_IntToString` (`KismetMathLibrary.FTrunc` _hours)) " : " (`KismetStringLibrary.Conv_IntToString` (`KismetMathLibrary.FTrunc` (- _returnvalue _minutes_2))))))

(fn `UpdateSuspision`
  (bind _deltatime (`self.DeltaTime`))
  (bind _suspicion (`self.Suspicion`))
  (if (`self.IsDealInProgress`)
    (set `self.Suspicion` (+ _deltatime _suspicion))
    (else
      (set `self.Suspicion` (- _suspicion _deltatime)))))

(fn `UpdateTime`
  (set `self.Time` (+ (`self.Time`) (* (`self.DeltaTime`) (`self.TimeScale`)))))

(fn `UserConstructionScript`)